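; Actor that receives positioning-tag messages through a Wutopia socket receiver and drives BP_CrossPawn movement.
; Each tick it reads one available message and stores X/Y/Z for four known tag IDs.
; Only pawns tagged for tag 000 are updated, with X/Y scaled by 100, rounded via text conversion, Z fixed, and values printed.
; Updates for the other three tags and debug-message handling are disconnected.
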(event EventBeginPlay
  (Class|WutopiaMsgReceiver|StartWutopiaMsgReceiver "BigSocket" 9088 -1 -1))

(event Collision|EventActorBeginOverlap
  (params (OtherActor :type Actor%20Object%20Reference)))

(event EventTick
  (params (DeltaSeconds :type Float%20%28single-precision%29))
  (bind _returnvalue (Class|WutopiaMsgReceiver|IsStarted))
  (if _returnvalue
    (bind _returnvalue_2 (Class|WutopiaMsgReceiver|IsConnected))
    (if _returnvalue_2
      (bind _returnvalue_3 (Class|WutopiaMsgReceiver|IsMsgAvailable))
      (if _returnvalue_3
        (bind _returnvalue_4 (Class|WutopiaMsgReceiver|GetData))
        (bind _output_get (Variables|Default|SetData _returnvalue_4))
        (switch string (.type (Utilities|Struct|BreakWutopiaData _output_get))
          (:TagBag
            (switch string (.tid (Utilities|Struct|BreakWutopiaTagBag (.TagBag (Utilities|Struct|BreakWutopiaData _output_get))))
              (:cn-hn-cs-kf-mgrc01-000
                (Variables|TagVector|SetX_0 (.x (Utilities|Struct|BreakWutopiaTagBag (.TagBag (Utilities|Struct|BreakWutopiaData _output_get)))))
                (Variables|TagVector|SetY_0 (.y (Utilities|Struct|BreakWutopiaTagBag (.TagBag (Utilities|Struct|BreakWutopiaData _output_get)))))
                (Variables|TagVector|SetZ_0 (.z (Utilities|Struct|BreakWutopiaTagBag (.TagBag (Utilities|Struct|BreakWutopiaData _output_get))))))
              (:cn-hn-cs-kf-mgrc01-005
                (Variables|TagVector|SetX_5 (.x (Utilities|Struct|BreakWutopiaTagBag (.TagBag (Utilities|Struct|BreakWutopiaData _output_get)))))
                (Variables|TagVector|SetY_5 (.y (Utilities|Struct|BreakWutopiaTagBag (.TagBag (Utilities|Struct|BreakWutopiaData _output_get)))))
                (Variables|TagVector|SetZ_5 (.z (Utilities|Struct|BreakWutopiaTagBag (.TagBag (Utilities|Struct|BreakWutopiaData _output_get))))))
              (:cn-hn-cs-kf-mgrc01-008
                (Variables|TagVector|SetX_8 (.x (Utilities|Struct|BreakWutopiaTagBag (.TagBag (Utilities|Struct|BreakWutopiaData _output_get)))))
                (Variables|TagVector|SetY_8 (.y (Utilities|Struct|BreakWutopiaTagBag (.TagBag (Utilities|Struct|BreakWutopiaData _output_get)))))
                (Variables|TagVector|SetZ_8 (.z (Utilities|Struct|BreakWutopiaTagBag (.TagBag (Utilities|Struct|BreakWutopiaData _output_get))))))
              (:cn-hn-cs-kf-mgrc01-010
                (Variables|TagVector|SetX_10 (.x (Utilities|Struct|BreakWutopiaTagBag (.TagBag (Utilities|Struct|BreakWutopiaData _output_get)))))
                (Variables|TagVector|SetY_10 (.y (Utilities|Struct|BreakWutopiaTagBag (.TagBag (Utilities|Struct|BreakWutopiaData _output_get)))))
                (Variables|TagVector|SetZ_10 (.z (Utilities|Struct|BreakWutopiaTagBag (.TagBag (Utilities|Struct|BreakWutopiaData _output_get)))))))
            (bind _outactors (Actor|GetAllActorsOfClass "/Game/_Cross/Blueprints/BP_CrossPawn.BP_CrossPawn_C"))
            (for _array_element _outactors
              (if (Actor|ActorHasTag _array_element "cn-hn-cs-kf-mgrc01-000")
                (Class|INTCrossTag|UpdateLocation(Message) _array_element (Math|Conversions|ToFloat(Integer) (Utilities|String|ToString(Text) (Utilities|Text|ToText(Float) (* (Variables|TagVector|GetX_0) 1e+02) "HalfToEven" false true 2 5 0 0))) (Math|Conversions|ToFloat(Integer) (Utilities|String|ToString(Text) (Utilities|Text|ToText(Float) (* (Variables|TagVector|GetY_0) 1e+02) "HalfToEven" false true 2 5 0 0))) 1.8e+02)
                (Development|PrintString (Utilities|String|Append (Utilities|String|MakeLiteralString "X:") (Utilities|String|ToString(Float) (Math|Conversions|ToFloat(Integer) (Utilities|String|ToString(Text) (Utilities|Text|ToText(Float) (* (Variables|TagVector|GetX_0) 1e+02) "HalfToEven" false true 2 5 0 0))))))
                (Development|PrintString (Utilities|String|Append (Utilities|String|MakeLiteralString "Y:") (Utilities|String|ToString(Float) (Math|Conversions|ToFloat(Integer) (Utilities|String|ToString(Text) (Utilities|Text|ToText(Float) (* (Variables|TagVector|GetY_0) 1e+02) "HalfToEven" false true 2 5 0 0))))))))))))))

(fn ConstructionScript)