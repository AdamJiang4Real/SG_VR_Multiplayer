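; BP_MyCrossbow is a single-shot crossbow actor with right-hand controller haptics.
; Reload, also run at BeginPlay, plays animation and sound, then after a short delay spawns a BP_MyBolt on the mesh's Bolt socket and enables firing.
; Fire detaches and shoots that bolt with animation, sound and haptics, emptying the ammo.
; Functions expose fire and reload, toggle Bolt component visibility, and cycle material variations.
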(event Custom|Reload
  ;[1 1 1] Reload
  (Variables|Default|SetAmmo 1)
  (Components|Animation|PlayAnimation (Variables|Default|GetCrossbow) "/Game/LightCrossbow/Meshes/Crossbow/Anim_Reload.Anim_Reload" false)
  (Audio|PlaySoundatLocation "/Game/VR_Archery/Audios/A_PullBack.A_PullBack" (Transformation|GetActorLocation) "0, 0, 0" 1.0 1.0 0.0 0 0 0 0) ; Play firing sound
  (Utilities|FlowControl|Delay 0.2)
  (bind _returnvalue (Game|SpawnActorfromClass "/Game/LightCrossbow/Blueprints/BP_MyBolt.BP_MyBolt_C" (Math|Transform|MakeTransform "0, 0, 0") "Undefined" "OverrideRootScale" 0 0))
  (bind _output_get (Variables|Default|SetMyBolt _returnvalue))
  (Transformation|AttachComponentToComponent _output_get (Variables|Default|GetCrossbow) "Bolt" "KeepRelative" "KeepRelative" "KeepRelative" true)
  (Variables|Default|SetbCanFire true)
  (Class|PlayerController|PlayHapticEffect (Game|GetPlayerController 0) "/Game/VR_Archery/Curve/ECurve_HandShock.ECurve_HandShock" "Right" 1.0 false))

(event Custom|Fire
  (bind _mybolt (Variables|Default|GetMyBolt))
  ;[1 1 1] Fire crossbow
  (if (and (> (Variables|Default|GetAmmo) 0) (Variables|Default|GetbCanFire))
    (Variables|Default|SetbCanFire false)
    (Transformation|DetachFromActor _mybolt "KeepWorld" "KeepWorld" "KeepWorld")
    (Default|Shoot _mybolt 0.0)
    (Audio|PlaySoundatLocation "/Game/LightCrossbow/Sounds/S_Ballista_Fire.S_Ballista_Fire" (Transformation|GetActorLocation) "0, 0, 0" 1.0 1.0 0.0 0 0 0 0) ; Play firing sound
    (Components|Animation|PlayAnimation (Variables|Default|GetCrossbow) "/Game/LightCrossbow/Meshes/Crossbow/Anim_Fire.Anim_Fire" false)
    (Variables|Default|SetAmmo 0)
    (Class|PlayerController|PlayHapticEffect (Game|GetPlayerController 0) "/Game/VR_Archery/Curve/ECurve_Shoot.ECurve_Shoot" "Right" 1.0 false)))

(event EventBeginPlay
  ;[1 1 1] Setup
  (CallFunction|Reload))

(fn ConstructionScript)

(fn SetBoltVisibility
  (params (Visible :type Boolean))
  ;[1 1 1] Show or hide the bolt
  (Rendering|SetVisibility (Variables|Default|GetBolt) Visible false))

(fn TryFire
  ;[1 1 1] Fire crossbow
  (CallFunction|Fire)
  (return true))

(fn TryReload
  ;[1 1 1] Start reload
  (CallFunction|Reload)
  (return true))

(fn SwitchMaterial
  ;[1 1 1] Switch Material
  (Math|Integer|IncrementInt (Variables|Default|GetMatIdx)
    (:%20%20
      (if (>= (Variables|Default|GetMatIdx) (Utilities|Array|Length (Variables|Default|GetMaterialVariations)))
        (Variables|Default|SetMatIdx 0))
      (Rendering|Material|SetMaterial (Variables|Default|GetCrossbow) 0 (Utilities|Array|Get(acopy) (Variables|Default|GetMaterialVariations) (Variables|Default|GetMatIdx))))))