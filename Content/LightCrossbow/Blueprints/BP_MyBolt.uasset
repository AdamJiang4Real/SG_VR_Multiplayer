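; Crossbow bolt projectile, fired through Shoot, which activates low-gravity projectile movement with rotation following velocity.
; A timeline scales the bolt for visibility until an overlap calls Stop, which ignores crossbow and pawn, resets scale and removes particles.
; Overlapped physics-simulating components receive a forward impulse and the bolt attaches to their actor.
; Line-trace damage and movement-stopping nodes are unconnected, and Destroy removes the actor after a delay.
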(event OnComponentBeginOverlap(BoltMesh)
  (params (OverlappedComponent :type Primitive%20Component%20Object%20Reference) (OtherActor :type Actor%20Object%20Reference) (OtherComp :type Primitive%20Component%20Object%20Reference) (OtherBodyIndex :type Integer) (bFromSweep :type Boolean) (SweepResult :type Hit%20Result%20Structure%20%28by%20ref%29))
  (bind _boltmesh (Variables|Default|GetBoltMesh))
  ;[1 1 1] Attach the bolt to the target that was hit and stop the movement
  (CallFunction|Stop OtherActor)
  (if (Class|SceneComponent|IsAnySimulatingPhysics OtherComp)
    (Physics|AddImpulseatLocation OtherComp (* (Math|Vector|GetForwardVector _boltmesh) 1e+05) (Transformation|GetWorldLocation _boltmesh) "None")
    (Transformation|AttachActorToActor OtherActor "None" "KeepWorld" "KeepWorld" "KeepWorld" true)))

(event Custom|StopRescaling
  ;[1 1 1] Scaling over time for visibility
  (bind _scale (Timeline|Timeline_0 Stop)
    (:Update
      (Transformation|SetRelativeScale3D (Variables|Default|GetRoot) (Math|Vector|MakeVector _scale _scale _scale)))))

(event Custom|Shoot
  (params (Speed :type Float%20%28double-precision%29))
  (bind _new_velocity_x (Variables|Default|GetNew%20Velocity%20X))
  (bind _projectilemovement (Variables|Default|GetProjectileMovement))
  (Game|Components|ProjectileMovement|SetVelocityinLocalSpace (Variables|Default|GetProjectileMovement) (Math|Vector|MakeVector _new_velocity_x 0.0 0.0))
  (Variables|/Script/Engine.ProjectileMovementComponent|SetInitialSpeed _projectilemovement _new_velocity_x)
  (Variables|/Script/Engine.ProjectileMovementComponent|SetMaxSpeed _projectilemovement _new_velocity_x)
  (Variables|/Script/Engine.ProjectileMovementComponent|SetProjectileGravityScale _projectilemovement 0.1)
  (Variables|/Script/Engine.ProjectileMovementComponent|SetbRotationFollowsVelocity (Variables|Default|GetProjectileMovement) true)
  (Components|Activation|SetActive (Variables|Default|GetProjectileMovement) true false))

(event Custom|Destroy
  (Utilities|FlowControl|Delay 3.0)
  (Actor|DestroyActor))

(event EventTick
  (params (DeltaSeconds :type Float%20%28single-precision%29)))

(event EventBeginPlay
  ;[1 1 1] Scaling over time for visibility
)

(fn ConstructionScript)

(fn Stop
  (params (OtherActor :type Actor%20Object%20Reference))
  (bind _particlesystem (Variables|Default|GetParticleSystem))
  ;[1 1 1] Ignore fpchar and crossbow so botl doesn't get stuck
  (Utilities|Casting|CastToBP_MyCrossbow OtherActor
    (:CastFailed
      (Utilities|Casting|CastToBP_CrossPawn OtherActor
        (:CastFailed
          ;[1 1 1] Reset scale
          (CallFunction|StopRescaling)
          (Transformation|SetWorldScale3D (Variables|Default|GetRoot) "1.000000,1.000000,1.000000")
          ;[1 1 1] Destroy particles
          (Utilities|IsValid _particlesystem
            (:Is%20Valid
              (Components|DestroyComponent _particlesystem))))))))