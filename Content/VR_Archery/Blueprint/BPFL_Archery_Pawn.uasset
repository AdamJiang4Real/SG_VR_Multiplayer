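; Blueprint function library for the VR archery pawn that drives hand animation.
; SetHandAnimation takes the first child component of a motion controller as the hand skeletal mesh and casts its anim instance to ABP_Hand.
; It then writes the grip state and the arrow-hand-to-notch value into that anim blueprint, silently stopping if either cast fails.
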(fn SetHandAnimation
  (params (HandAnimation :type E_GripEnum%20Enum :default "NewEnumerator0") (HoldingController :type Motion%20Controller%20Component%20Object%20Reference) (ArrowHandToNotch :type Float%20%28double-precision%29))
  (LocalVariables|SetAnimation HandAnimation)
  (bind _output_get (LocalVariables|SetNewLocalVar HoldingController))
  (LocalVariables|SetDistance ArrowHandToNotch)
  (bind _as骨骼网格体组件 (Utilities|Casting|CastToSkeletalMeshComponent (Components|GetChildComponent _output_get 0)))
  (bind _asabp_hand (Utilities|Casting|CastToABP_Hand (Components|SkeletalMesh|GetAnimInstance _as骨骼网格体组件)))
  (Variables|/Game/VR_Archery/Animations/Hand/ABP_Hand.ABP_Hand_C|SetGripState _asabp_hand (LocalVariables|GetAnimation))
  (Variables|/Game/VR_Archery/Animations/Hand/ABP_Hand.ABP_Hand_C|SetArrowHandToNotch _asabp_hand (LocalVariables|GetDistance)))