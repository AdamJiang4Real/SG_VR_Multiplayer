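; Enemy character for a VR archery game that disappears for a few seconds and then reappears, rather than being removed.
; A capsule overlap with a component named like "ArrowBox" passes the enemy to SetEnemyVisibility on every VR_Pawn.
; Its Destroy event hides the mesh and disables collision, then restores both as query-only collision and visible mesh after a delay.
; The bDisappear replication handler is empty, with leftover hide logic left unconnected.
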(event OnComponentBeginOverlap(CapsuleComponent)
  (params (OverlappedComponent :type Primitive%20Component%20Object%20Reference) (OtherActor :type Actor%20Object%20Reference) (OtherComp :type Primitive%20Component%20Object%20Reference) (OtherBodyIndex :type Integer) (bFromSweep :type Boolean) (SweepResult :type Hit%20Result%20Structure%20%28by%20ref%29))
  (if (Utilities|String|Contains (Utilities|GetDisplayName OtherComp) "ArrowBox")
    (bind _outactors (Actor|GetAllActorsOfClass "/Game/VR_Archery/Blueprint/VR_Pawn.VR_Pawn_C"))
    (for _array_element _outactors
      (Default|SetEnemyVisibility _array_element self))))

(event Custom|Destroy
  (bind _mesh (Variables|Character|GetMesh))
  (Development|PrintString "Client Destroy")
  (Rendering|SetVisibility (Variables|Character|GetMesh) false false)
  (Rendering|SetVisibility (Variables|Character|GetMesh) false true)
  (Collision|SetCollisionEnabled (Variables|Character|GetMesh) "NoCollision")
  (Utilities|FlowControl|Delay 3.0)
  (Rendering|SetVisibility _mesh true true)
  (Collision|SetCollisionEnabled _mesh "QueryOnly"))

(event EventBeginPlay)

(fn ConstructionScript)

(fn OnRepBDisappear)