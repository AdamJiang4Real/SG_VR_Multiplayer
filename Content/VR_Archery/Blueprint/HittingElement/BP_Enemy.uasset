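; BP_Enemy is an archery target in the VR Archery game that detects arrows through a box overlap on components named like ArrowBox.
; A hit runs a client-to-server event chain, which currently only prints debug text and passes an empty arrow reference.
; A multicast event hides the arrow and target, then restores the target after a delay, but its calls are disconnected.
; Random material refresh is also unwired.
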(event OnComponentBeginOverlap(Box)
  (params (OverlappedComponent :type Primitive%20Component%20Object%20Reference) (OtherActor :type Actor%20Object%20Reference) (OtherComp :type Primitive%20Component%20Object%20Reference) (OtherBodyIndex :type Integer) (bFromSweep :type Boolean) (SweepResult :type Hit%20Result%20Structure%20%28by%20ref%29))
  (bind _output_get (Variables|Default|SetOther%20Actor OtherActor))
  (if (Utilities|String|Contains (Utilities|GetDisplayName OtherComp) "ArrowBox")
    (Utilities|Casting|CastToBP_Arrow _output_get)
    (bind _output_get_2 (Variables|Default|SetAs%20BP%20Arrow 0))
    (CallFunction|ClientCall _output_get_2)))

(event Custom|Server_Destroy
  (params (Arrow :type BP%20Arrow%20Object%20Reference))
  (Utilities|IsValid Arrow
    (:Is%20Valid
      (Development|PrintString (Utilities|GetDisplayName Arrow)))
    (:Is%20Not%20Valid
      (Development|PrintString "Server No Target"))))

(event Custom|Multicast_Destroy
  (params (As%20BP%20Arrow :type BP%20Arrow%20Object%20Reference))
  (Rendering|SetVisibility (Variables|/Script/Engine.Actor|GetRootComponent As%20BP%20Arrow) false false)
  (Collision|SetCollisionEnabled (Variables|/Game/VR_Archery/Blueprint/BowAndArrow/BP_Arrow.BP_Arrow_C|GetArrowBox As%20BP%20Arrow) "NoCollision")
  (Rendering|SetVisibility (Variables|Default|GetSkeletalMesh) false true)
  (Collision|SetCollisionEnabled (Variables|Default|GetSkeletalMesh) "NoCollision")
  (Utilities|FlowControl|Delay 2.0)
  (Rendering|SetVisibility (Variables|Default|GetSkeletalMesh) true true)
  (Collision|SetCollisionEnabled (Variables|Default|GetSkeletalMesh) "QueryOnly"))

(event Custom|Client_Call
  (params (As%20BP%20Arrow :type BP%20Arrow%20Object%20Reference))
  (CallFunction|ServerDestroy As%20BP%20Arrow)
  (Development|PrintString "Client Call"))

(fn ConstructionScript)

(fn RefreshMaterial)