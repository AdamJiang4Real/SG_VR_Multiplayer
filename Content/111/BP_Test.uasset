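; BP_Test is a test actor with a Cube that rises on a timeline.
; BeginPlay stores the Cube's world position, and the Multi_Server_Rise event lerps its height from there to a fixed world Z, then snaps it back when the timeline finishes.
; The Sphere overlap casts to BP_ThirdPersonCharacter but does nothing afterward, and nothing in this file calls the rise event.
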(event OnComponentBeginOverlap(Sphere)
  (params (OverlappedComponent :type Primitive%20Component%20Object%20Reference) (OtherActor :type Actor%20Object%20Reference) (OtherComp :type Primitive%20Component%20Object%20Reference) (OtherBodyIndex :type Integer) (bFromSweep :type Boolean) (SweepResult :type Hit%20Result%20Structure%20%28by%20ref%29))
  (Utilities|Casting|CastToBP_ThirdPersonCharacter OtherActor))

(event Custom|Multi_Server_Rise
  (bind _newtrack_0 (Timeline|Timeline PlayFromStart)
    (:Update
      (Transformation|SetWorldLocation (Variables|Default|GetCube) (Math|Vector|MakeVector (Variables|Default|GetValue%20X_0) (Variables|Default|GetValue%20Y_0) (Math|Float|Lerp (Variables|Default|GetValue%20Z_0) 8e+02 _newtrack_0)) false false))
    (:Finished
      (Transformation|SetWorldLocation (Variables|Default|GetCube) (Math|Vector|MakeVector (Variables|Default|GetValue%20X_0) (Variables|Default|GetValue%20Y_0) (Variables|Default|GetValue%20Z_0)) false false))))

(event EventBeginPlay
  (bind _cube (Variables|Default|GetCube))
  (bind _returnvalue (Transformation|GetWorldLocation _cube))
  (Variables|Default|SetValue%20X_0 (.x _returnvalue))
  (Variables|Default|SetValue%20Y_0 (.y _returnvalue))
  (Variables|Default|SetValue%20Z_0 (.z _returnvalue)))

(event Collision|EventActorBeginOverlap
  (params (OtherActor :type Actor%20Object%20Reference)))

(event EventTick
  (params (DeltaSeconds :type Float%20%28single-precision%29)))

(fn ConstructionScript)