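; BP_Kong is an interactable mesh actor that floats upward when Rise is triggered, then resets to its start position.
; Its sphere tells a VR_Pawn to set or clear its target flag as a GrabSphere component enters or leaves.
; Rise, labeled server multicast, runs a guarded timeline that lerps world Z from the BeginPlay position to a fixed height.
; Third-person overlap logic remains but is disconnected.
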(event OnComponentBeginOverlap(Sphere)
  (params (OverlappedComponent :type Primitive%20Component%20Object%20Reference) (OtherActor :type Actor%20Object%20Reference) (OtherComp :type Primitive%20Component%20Object%20Reference) (OtherBodyIndex :type Integer) (bFromSweep :type Boolean) (SweepResult :type Hit%20Result%20Structure%20%28by%20ref%29))
  ;[1 1 1] Begin Overlapped
  ;;[0 0.05363 1] VR
  (if (Utilities|String|Contains (Utilities|GetDisplayName OtherComp) "GrabSphere")
    (bind _asvr_pawn (Utilities|Casting|CastToVR_Pawn OtherActor))
    (bind _output_get (Variables|Default|SetAs%20VR%20Pawn _asvr_pawn))
    (Default|SetTarget _output_get true)))

(event OnComponentEndOverlap(Sphere)
  (params (OverlappedComponent :type Primitive%20Component%20Object%20Reference) (OtherActor :type Actor%20Object%20Reference) (OtherComp :type Primitive%20Component%20Object%20Reference) (OtherBodyIndex :type Integer))
  ;[1 1 1] End Overlapped
  ;;[0 0.05363 1] VR
  (if (Utilities|String|Contains (Utilities|GetDisplayName OtherComp) "GrabSphere")
    (bind _asvr_pawn (Utilities|Casting|CastToVR_Pawn OtherActor))
    (bind _output_get (Variables|Default|SetAs%20VR%20Pawn _asvr_pawn))
    (Default|SetTarget _output_get false)))

(event Custom|Rise
  (bind _staticmesh (Variables|Default|GetStaticMesh))
  ;[1 1 1] Server Multicast
  (Development|PrintString "Client Rising........" true true "(R=1.000000,G=0.077258,B=0.000000,A=1.000000)" 5.0)
  (if (not (Variables|Default|GetbIsRunning?))
    (Variables|Default|SetbIsRunning? true)
    (bind _新建轨道_2 (Timeline|时间轴 PlayFromStart)
      (:Update
        (Transformation|SetWorldLocation _staticmesh (Math|Vector|MakeVector (Variables|Default|GetValue%20X_0) (Variables|Default|GetValue%20Y_0) (Math|Float|Lerp (Variables|Default|GetValue%20Z_0) 8e+02 _新建轨道_2)) false false))
      (:Finished
        (Rendering|SetVisibility _staticmesh false false)
        (Transformation|SetWorldLocation (Variables|Default|GetStaticMesh) (Math|Vector|MakeVector (Variables|Default|GetValue%20X_0) (Variables|Default|GetValue%20Y_0) (Variables|Default|GetValue%20Z_0)) false false)
        (Rendering|SetVisibility (Variables|Default|GetStaticMesh) true false)
        (Variables|Default|SetbIsRunning? false)))))

(event EventBeginPlay
  (bind _staticmesh (Variables|Default|GetStaticMesh))
  (bind _returnvalue (Transformation|GetWorldLocation _staticmesh))
  ;[1 1 1] 注释
  (Variables|Default|SetValue%20X_0 (.x _returnvalue))
  (Variables|Default|SetValue%20Y_0 (.y _returnvalue))
  (Variables|Default|SetValue%20Z_0 (.z _returnvalue)))

(event Collision|EventActorBeginOverlap
  (params (OtherActor :type Actor%20Object%20Reference)))

(fn ConstructionScript)