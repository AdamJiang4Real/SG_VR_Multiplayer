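; BP_Bazi is a shooting target that scores crossbow bolt hits across ten zones worth 1 to 10 points.
; Each zone's overlap calls Shoot, which recognizes the bolt by mesh display name, stops it, updates Score and destroys it.
; Two text renders show the last hit's score and the running total.
; Bolt overlaps on either SM_Kong mesh reset the total to zero without destroying the bolt.
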(event OnComponentBeginOverlap(SM_Kong)
  (params (OverlappedComponent :type Primitive%20Component%20Object%20Reference) (OtherActor :type Actor%20Object%20Reference) (OtherComp :type Primitive%20Component%20Object%20Reference) (OtherBodyIndex :type Integer) (bFromSweep :type Boolean) (SweepResult :type Hit%20Result%20Structure%20%28by%20ref%29))
  (if (Utilities|String|Contains (Utilities|GetDisplayName OtherComp) "SM_Bolt_01")
    (Variables|Default|SetScore 0)
    (Rendering|Components|TextRender|SetText (Variables|Default|GetTextRender_02) (Utilities|Text|ToText(String) (Utilities|String|Append (Utilities|String|MakeLiteralString "Total:   ") (Utilities|String|ToString(Integer) (Variables|Default|GetScore)))))
    (Rendering|Components|TextRender|SetText (Variables|Default|GetTextRender) (Utilities|Text|FormatText "Score:   0"))))

(event OnComponentBeginOverlap(SM_Kong_02)
  (params (OverlappedComponent :type Primitive%20Component%20Object%20Reference) (OtherActor :type Actor%20Object%20Reference) (OtherComp :type Primitive%20Component%20Object%20Reference) (OtherBodyIndex :type Integer) (bFromSweep :type Boolean) (SweepResult :type Hit%20Result%20Structure%20%28by%20ref%29))
  (if (Utilities|String|Contains (Utilities|GetDisplayName OtherComp) "SM_Bolt_01")
    (Variables|Default|SetScore 0)
    (Rendering|Components|TextRender|SetText (Variables|Default|GetTextRender_02) (Utilities|Text|ToText(String) (Utilities|String|Append (Utilities|String|MakeLiteralString "Total:   ") (Utilities|String|ToString(Integer) (Variables|Default|GetScore)))))
    (Rendering|Components|TextRender|SetText (Variables|Default|GetTextRender) (Utilities|Text|FormatText "Score:   0"))))

(event OnComponentBeginOverlap(1)
  (params (OverlappedComponent :type Primitive%20Component%20Object%20Reference) (OtherActor :type Actor%20Object%20Reference) (OtherComp :type Primitive%20Component%20Object%20Reference) (OtherBodyIndex :type Integer) (bFromSweep :type Boolean) (SweepResult :type Hit%20Result%20Structure%20%28by%20ref%29))
  (bind _isshoot (CallFunction|Shoot OtherActor OtherComp 1))
  (if _isshoot
    (Rendering|Components|TextRender|SetText (Variables|Default|GetTextRender) (Utilities|Text|FormatText "Score:   1"))
    (Rendering|Components|TextRender|SetText (Variables|Default|GetTextRender_02) (Utilities|Text|ToText(String) (Utilities|String|Append (Utilities|String|MakeLiteralString "Total:   ") (Utilities|String|ToString(Integer) (Variables|Default|GetScore)))))))

(event OnComponentBeginOverlap(2)
  (params (OverlappedComponent :type Primitive%20Component%20Object%20Reference) (OtherActor :type Actor%20Object%20Reference) (OtherComp :type Primitive%20Component%20Object%20Reference) (OtherBodyIndex :type Integer) (bFromSweep :type Boolean) (SweepResult :type Hit%20Result%20Structure%20%28by%20ref%29))
  (bind _isshoot (CallFunction|Shoot OtherActor OtherComp 2))
  (if _isshoot
    (Rendering|Components|TextRender|SetText (Variables|Default|GetTextRender) (Utilities|Text|FormatText "Score:   2"))
    (Rendering|Components|TextRender|SetText (Variables|Default|GetTextRender_02) (Utilities|Text|ToText(String) (Utilities|String|Append (Utilities|String|MakeLiteralString "Total:   ") (Utilities|String|ToString(Integer) (Variables|Default|GetScore)))))))

(event OnComponentBeginOverlap(3)
  (params (OverlappedComponent :type Primitive%20Component%20Object%20Reference) (OtherActor :type Actor%20Object%20Reference) (OtherComp :type Primitive%20Component%20Object%20Reference) (OtherBodyIndex :type Integer) (bFromSweep :type Boolean) (SweepResult :type Hit%20Result%20Structure%20%28by%20ref%29))
  (bind _isshoot (CallFunction|Shoot OtherActor OtherComp 3))
  (if _isshoot
    (Rendering|Components|TextRender|SetText (Variables|Default|GetTextRender) (Utilities|Text|FormatText "Score:   3"))
    (Rendering|Components|TextRender|SetText (Variables|Default|GetTextRender_02) (Utilities|Text|ToText(String) (Utilities|String|Append (Utilities|String|MakeLiteralString "Total:   ") (Utilities|String|ToString(Integer) (Variables|Default|GetScore)))))))

(event OnComponentBeginOverlap(4)
  (params (OverlappedComponent :type Primitive%20Component%20Object%20Reference) (OtherActor :type Actor%20Object%20Reference) (OtherComp :type Primitive%20Component%20Object%20Reference) (OtherBodyIndex :type Integer) (bFromSweep :type Boolean) (SweepResult :type Hit%20Result%20Structure%20%28by%20ref%29))
  (bind _isshoot (CallFunction|Shoot OtherActor OtherComp 4))
  (if _isshoot
    (Rendering|Components|TextRender|SetText (Variables|Default|GetTextRender) (Utilities|Text|FormatText "Score:   4"))
    (Rendering|Components|TextRender|SetText (Variables|Default|GetTextRender_02) (Utilities|Text|ToText(String) (Utilities|String|Append (Utilities|String|MakeLiteralString "Total:   ") (Utilities|String|ToString(Integer) (Variables|Default|GetScore)))))))

(event OnComponentBeginOverlap(5)
  (params (OverlappedComponent :type Primitive%20Component%20Object%20Reference) (OtherActor :type Actor%20Object%20Reference) (OtherComp :type Primitive%20Component%20Object%20Reference) (OtherBodyIndex :type Integer) (bFromSweep :type Boolean) (SweepResult :type Hit%20Result%20Structure%20%28by%20ref%29))
  (bind _isshoot (CallFunction|Shoot OtherActor OtherComp 5))
  (if _isshoot
    (Rendering|Components|TextRender|SetText (Variables|Default|GetTextRender) (Utilities|Text|FormatText "Score:   5"))
    (Rendering|Components|TextRender|SetText (Variables|Default|GetTextRender_02) (Utilities|Text|ToText(String) (Utilities|String|Append (Utilities|String|MakeLiteralString "Total:   ") (Utilities|String|ToString(Integer) (Variables|Default|GetScore)))))))

(event OnComponentBeginOverlap(6)
  (params (OverlappedComponent :type Primitive%20Component%20Object%20Reference) (OtherActor :type Actor%20Object%20Reference) (OtherComp :type Primitive%20Component%20Object%20Reference) (OtherBodyIndex :type Integer) (bFromSweep :type Boolean) (SweepResult :type Hit%20Result%20Structure%20%28by%20ref%29))
  (bind _isshoot (CallFunction|Shoot OtherActor OtherComp 6))
  (if _isshoot
    (Rendering|Components|TextRender|SetText (Variables|Default|GetTextRender) (Utilities|Text|FormatText "Score:   6"))
    (Rendering|Components|TextRender|SetText (Variables|Default|GetTextRender_02) (Utilities|Text|ToText(String) (Utilities|String|Append (Utilities|String|MakeLiteralString "Total:   ") (Utilities|String|ToString(Integer) (Variables|Default|GetScore)))))))

(event OnComponentBeginOverlap(7)
  (params (OverlappedComponent :type Primitive%20Component%20Object%20Reference) (OtherActor :type Actor%20Object%20Reference) (OtherComp :type Primitive%20Component%20Object%20Reference) (OtherBodyIndex :type Integer) (bFromSweep :type Boolean) (SweepResult :type Hit%20Result%20Structure%20%28by%20ref%29))
  (bind _isshoot (CallFunction|Shoot OtherActor OtherComp 7))
  (if _isshoot
    (Rendering|Components|TextRender|SetText (Variables|Default|GetTextRender) (Utilities|Text|FormatText "Score:   7"))
    (Rendering|Components|TextRender|SetText (Variables|Default|GetTextRender_02) (Utilities|Text|ToText(String) (Utilities|String|Append (Utilities|String|MakeLiteralString "Total:   ") (Utilities|String|ToString(Integer) (Variables|Default|GetScore)))))))

(event OnComponentBeginOverlap(8)
  (params (OverlappedComponent :type Primitive%20Component%20Object%20Reference) (OtherActor :type Actor%20Object%20Reference) (OtherComp :type Primitive%20Component%20Object%20Reference) (OtherBodyIndex :type Integer) (bFromSweep :type Boolean) (SweepResult :type Hit%20Result%20Structure%20%28by%20ref%29))
  (bind _isshoot (CallFunction|Shoot OtherActor OtherComp 8))
  (if _isshoot
    (Rendering|Components|TextRender|SetText (Variables|Default|GetTextRender) (Utilities|Text|FormatText "Score:   8"))
    (Rendering|Components|TextRender|SetText (Variables|Default|GetTextRender_02) (Utilities|Text|ToText(String) (Utilities|String|Append (Utilities|String|MakeLiteralString "Total:   ") (Utilities|String|ToString(Integer) (Variables|Default|GetScore)))))))

(event OnComponentBeginOverlap(9)
  (params (OverlappedComponent :type Primitive%20Component%20Object%20Reference) (OtherActor :type Actor%20Object%20Reference) (OtherComp :type Primitive%20Component%20Object%20Reference) (OtherBodyIndex :type Integer) (bFromSweep :type Boolean) (SweepResult :type Hit%20Result%20Structure%20%28by%20ref%29))
  (bind _isshoot (CallFunction|Shoot OtherActor OtherComp 9))
  (if _isshoot
    (Rendering|Components|TextRender|SetText (Variables|Default|GetTextRender) (Utilities|Text|FormatText "Score:   9"))
    (Rendering|Components|TextRender|SetText (Variables|Default|GetTextRender_02) (Utilities|Text|ToText(String) (Utilities|String|Append (Utilities|String|MakeLiteralString "Total:   ") (Utilities|String|ToString(Integer) (Variables|Default|GetScore)))))))

(event OnComponentBeginOverlap(10)
  (params (OverlappedComponent :type Primitive%20Component%20Object%20Reference) (OtherActor :type Actor%20Object%20Reference) (OtherComp :type Primitive%20Component%20Object%20Reference) (OtherBodyIndex :type Integer) (bFromSweep :type Boolean) (SweepResult :type Hit%20Result%20Structure%20%28by%20ref%29))
  (bind _isshoot (CallFunction|Shoot OtherActor OtherComp 10))
  (if _isshoot
    (Rendering|Components|TextRender|SetText (Variables|Default|GetTextRender) (Utilities|Text|FormatText "Score:   10"))
    (Rendering|Components|TextRender|SetText (Variables|Default|GetTextRender_02) (Utilities|Text|ToText(String) (Utilities|String|Append (Utilities|String|MakeLiteralString "Total:   ") (Utilities|String|ToString(Integer) (Variables|Default|GetScore)))))))

(fn ConstructionScript)

(fn Shoot
  (params (OtherActor :type Actor%20Object%20Reference) (OtherComponent :type Scene%20Component%20Object%20Reference) (Score :type Integer))
  (if (Utilities|String|Contains (Utilities|GetDisplayName OtherComponent) "SM_Bolt_01")
    (bind _asbp_my_bolt (Utilities|Casting|CastToBP_MyBolt OtherActor))
    (Components|Movement|StopMovementImmediately (Variables|/Game/_Cross/Blueprints/BP_MyBolt.BP_MyBolt_C|GetProjectileMovement _asbp_my_bolt))
    (Components|Activation|SetActive (Variables|/Game/_Cross/Blueprints/BP_MyBolt.BP_MyBolt_C|GetProjectileMovement _asbp_my_bolt) false false)
    (Collision|SetCollisionEnabled (Variables|/Game/_Cross/Blueprints/BP_MyBolt.BP_MyBolt_C|GetBoltMesh _asbp_my_bolt) "NoCollision")
    (Variables|Default|SetScore (+ Score (Variables|Default|GetScore)))
    (Default|Destroy _asbp_my_bolt)
    (return true)
    (else
      (return false))))