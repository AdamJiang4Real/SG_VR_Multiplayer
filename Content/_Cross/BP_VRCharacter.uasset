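; Networked VR character pawn whose position is set from X, Y, Z coordinates and which carries a tag ID.
; On BeginPlay the authority spawns a BP_MainProcess owned by the character.
; UpdateLocation passes coordinates to a multicast event that moves the actor and capsule through SetActorLocationVR.
; It also sends the ID to a server event, which stores it and adds non-empty values to the actor's tags.
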(event Custom|SERVER_GetTid
  (params (Tid :type String))
  (bind _actor_tags (Variables|Default|GetActor%20Tags))
  (bind _output_get (Variables|Default|SetTag%20ID Tid))
  (if (not (Utilities|Array|IsEmpty _output_get))
    (bind _output_get_2 (Variables|Default|SetTagID%20Name (Utilities|String|StringToName _output_get)))
    (Utilities|Array|AddUnique _actor_tags _output_get_2)
    (Variables|Default|SetTags _actor_tags)))

(event Custom|MULTI_UpdateLocation
  (params (X :type Float%20%28double-precision%29) (Y :type Float%20%28double-precision%29) (Z :type Float%20%28double-precision%29))
  (Class|VRBaseCharacter|SetActorLocationVR (Math|Vector|MakeVector X Y Z) false true))

(event EventUpdateLocation
  (params (X :type Float%20%28double-precision%29) (Y :type Float%20%28double-precision%29) (Z :type Float%20%28double-precision%29) (Tid :type String))
  (CallFunction|MULTIUpdateLocation X Y Z)
  (CallFunction|SERVERGetTid Tid))

(event EventBeginPlay
  (Networking|SwitchHasAuthority
    (:Authority
      (Game|SpawnActorfromClass "/Game/_TagMotion/Blueprints/BP_MainProcess.BP_MainProcess_C" (Math|Transform|MakeTransform "0, 0, 0") "Undefined" "MultiplyWithRoot" self 0))))

(fn ConstructionScript)