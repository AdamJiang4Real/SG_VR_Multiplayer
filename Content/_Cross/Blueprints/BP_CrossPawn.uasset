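; BP_CrossPawn is a networked VR player pawn that wields a crossbow in its right hand.
; BeginPlay spawns BP_MainProcess, sets headset-specific tracking origin, sends controller transforms once from remote instances and requests the crossbow.
; The right trigger messages the crossbow to fire or reload by ammo, while pawn events handle bolt attachment and launch.
; Server and multicast events drive spawning, animations, sound, haptics and enemy destruction.
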(event Custom|SERVER_SpawnCrossBow
  ;[0 0.3002 1] Spawn CrossBolt
  (Variables|Default|GetCrossBow
    (:then)
    (:else
      (bind _returnvalue (Game|SpawnActorfromClass "/Game/_Cross/Blueprints/BP_MyCrossbow.BP_MyCrossbow_C" (Math|Transform|MakeTransform "0, 0, 0" "0, 0, 0" "0.600000,0.600000,0.600000") "Undefined" "MultiplyWithRoot" 0 0))
      (bind _output_get (Variables|Default|SetCrossBow _returnvalue))
      (Actor|SetOwner _output_get self)
      (CallFunction|SERVERAttachCrossBow (Variables|Default|GetCrossBow)))))

(event Custom|SERVER_AttachCrossBow
  (params (CrossBow :type Actor%20Object%20Reference))
  ;[0 0.3002 1] Spawn CrossBolt
  (Utilities|IsValid CrossBow
    (:Is%20Valid
      (bind _skm_right (Variables|Default|GetSKM_Right)
        (:then
          (Transformation|AttachComponentToComponent (Variables|Default|GetCrossBow) _skm_right "Cross" "SnapToTarget" "SnapToTarget" "KeepRelative" false))
        (:else)))))

(event Custom|MULTI_Trigger
  (params (bTriggerPull :type Boolean))
  ;[0 0 0] Comment
  (Variables|Default|SetbTriggerPull bTriggerPull))

(event Custom|SERVER_Fire
  ;[1 0.07208 0] Fire
  (CallFunction|MULTIFire)
  (CallFunction|SERVERHaptic "/Game/VR_Archery/Curve/ECurve_Shoot.ECurve_Shoot"))

(event Custom|MULTI_Fire
  (bind _bolt (Variables|Default|GetBolt))
  ;[1 0.07208 0] Fire
  (bind _bolt_2 (Variables|Default|GetBolt)
    (:then
      (if (Variables|Default|GetIsBoltSet)
        (Transformation|DetachFromActor _bolt "KeepWorld" "KeepWorld" "KeepWorld")
        (Default|Shoot _bolt 1e+03)
        (Audio|PlaySoundatLocation "/Game/LightCrossbow/Sounds/S_Ballista_Fire.S_Ballista_Fire" (Transformation|GetWorldLocation (Variables|Default|GetMotionController_Right)) "0, 0, 0" 1.0 1.0 0.0 0 0 0 0) ; Play firing sound
        (Components|Animation|PlayAnimation (Variables|/Game/_Cross/Blueprints/BP_MyCrossbow.BP_MyCrossbow_C|GetCrossbowMesh (Variables|Default|GetCrossbolt)) "/Game/LightCrossbow/Meshes/Crossbow/Anim_Fire.Anim_Fire" false)
        (Variables|Default|SetIsBoltSet false)))
    (:else)))

(event Custom|SERVER_Haptic
  (params (HapticEffect :type Haptic%20Feedback%20Effect%20Base%20Object%20Reference))
  ;[0 1 0.2449] Spawn Bolt And Reload
  (bind _playercontroller (CallFunction|GetControllerfromPC))
  (Class|PlayerController|PlayHapticEffect _playercontroller HapticEffect "Right" 1.0 false))

(event Custom|SERVER_UpdateLeft
  (params (Transform :type Transform))
  ;[1 1 1] Comment
  (Transformation|SetWorldTransform (Variables|Default|GetMotionController_Left) Transform false false))

(event Custom|SERVER_UpdateRight
  (params (Transform :type Transform))
  ;[1 1 1] Comment
  (Transformation|SetWorldTransform (Variables|Default|GetMotionController_Right) Transform false false))

(event Custom|SERVER_SetEnemyVisibility
  (params (Enemy :type BP%20Enemy%20AI%20Object%20Reference) (Bolt :type BP%20My%20Bolt%20Object%20Reference))
  ;[1 0.4552 0.2226] Destroy Enemy
  (CallFunction|MULTIDestroy Enemy Bolt))

(event Custom|MULTI_Destroy
  (params (Enemy :type BP%20Enemy%20AI%20Object%20Reference) (Bolt :type BP%20My%20Bolt%20Object%20Reference))
  ;[1 0.4552 0.2226] Destroy Enemy
  (Default|Destroy Enemy)
  (Utilities|IsValid Bolt
    (:Is%20Valid
      (Default|DestroyNow Bolt))))

(event Custom|SERVER_EndPull
  ;[0 0 0] Comment
  (CallFunction|MULTITrigger false))

(event Custom|SERVER_BeginPull
  (bind _self self)
  (bind _crossbow (Variables|Default|GetCrossBow))
  (bind _crossbow_2 (Variables|Default|GetCrossBow))
  ;[0 0 0] Comment
  (if true
    (Utilities|IsValid _crossbow
      (:Is%20Valid
        (if (> (Variables|/Game/_Cross/Blueprints/BP_MyCrossbow.BP_MyCrossbow_C|GetAmmo _crossbow) 0)
          (Class|INTCrossBow|Fire(Message) _crossbow_2 _self)
          (else
            (Class|INTCrossBow|Reload(Message) _crossbow_2 _self)))
        (CallFunction|MULTITrigger true)))))

(event Custom|SERVER_UpdateTagLocation
  (params (X :type Float%20%28double-precision%29) (Y :type Float%20%28double-precision%29) (Z :type Float%20%28double-precision%29))
  (Transformation|SetActorLocation (Math|Vector|MakeVector X Y 9e+01) false false))

(event Custom|SERVER_SpawnAndPlayMontage
  (params (Crossbolt :type BP%20My%20Crossbow%20Object%20Reference))
  ;[0 1 0.2449] Spawn Bolt And Reload
  (bind _returnvalue (Game|SpawnActorfromClass "/Game/_Cross/Blueprints/BP_MyBolt.BP_MyBolt_C" (Math|Transform|MakeTransform "0, 0, 0") "Undefined" "OverrideRootScale" 0 0))
  (CallFunction|MULTIAttachBolt2Cross _returnvalue Crossbolt)
  (CallFunction|SERVERHaptic "/Game/VR_Archery/Curve/ECurve_HandShock.ECurve_HandShock"))

(event Custom|MULTI_AttachBolt2Cross
  (params (Bolt :type BP%20My%20Bolt%20Object%20Reference) (Crossbolt :type BP%20My%20Crossbow%20Object%20Reference))
  ;[0 1 0.2449] Spawn Bolt And Reload
  (Utilities|IsValid Bolt
    (:Is%20Valid
      (Variables|Default|SetBolt Bolt)
      (Utilities|IsValid Crossbolt
        (:Is%20Valid
          (bind _output_get (Variables|Default|SetCrossbolt Crossbolt))
          (Transformation|AttachComponentToComponent (Variables|Default|GetBolt) (Variables|/Game/_Cross/Blueprints/BP_MyCrossbow.BP_MyCrossbow_C|GetCrossbowMesh _output_get) "Bolt" "KeepRelative" "KeepRelative" "KeepRelative" true)
          (Components|Animation|PlayAnimation (Variables|/Game/_Cross/Blueprints/BP_MyCrossbow.BP_MyCrossbow_C|GetCrossbowMesh (Variables|Default|GetCrossbolt)) "/Game/LightCrossbow/Meshes/Crossbow/Anim_Reload.Anim_Reload" false)
          (Variables|Default|SetIsBoltSet true))))))

(event EventBeginPlay
  ;[1 1 1] Comment
  (Utilities|FlowControl|Sequence
    (:then_0
      (Game|SpawnActorfromClass "/Game/_TagMotion/Blueprints/BP_MainProcess.BP_MainProcess_C" (Math|Transform|MakeTransform "0, 0, 0" "0, 0, 0" "1.000000,1.000000,1.000000") "Undefined" "MultiplyWithRoot" self 0))
    (:then_1
      (switch name (Class|HeadMountedDisplayFunctionLibrary|GetHMDDeviceName)
        (:OculusHMD
          (Class|HeadMountedDisplayFunctionLibrary|SetTrackingOrigin "Floor" :!label _label) ; Windows (Oculus / Vive)
          ;[1 1 1] Comment
          (Networking|SwitchHasAuthority
            (:Remote
              (Utilities|FlowControl|Sequence
                (:then_0
                  (CallFunction|SERVERUpdateLeft (Transformation|GetWorldTransform (Variables|Default|GetMotionController_Left))))
                (:then_1
                  (CallFunction|SERVERUpdateRight (Transformation|GetWorldTransform (Variables|Default|GetMotionController_Right))))))))
        (:SteamVR
          (goto _label))
        (:PSVR
          (Class|HeadMountedDisplayFunctionLibrary|SetTrackingOrigin "Eye") ; PS4
          (Transformation|AddLocalOffset (Variables|Default|GetVROrigin) (Math|Vector|MakeVector 0.0 0.0 (Variables|Default|GetDefaultPlayerHeight)) false false))))
    (:then_2
      (CallFunction|SERVERSpawnCrossBow))))

(event EventUpdateLocation
  (params (Tid :type String) (X :type Float%20%28double-precision%29) (Y :type Float%20%28double-precision%29) (Z :type Float%20%28double-precision%29))
  (CallFunction|SERVERUpdateTagLocation X Y 0.0))

(event EventSpawnandPlayCrossMontage
  (params (BPCrossBow :type BP%20My%20Crossbow%20Object%20Reference))
  ;[0 1 0.2449] Spawn Bolt And Reload
  (if (not (Variables|Default|GetIsBoltSet))
    (CallFunction|SERVERSpawnandPlayMontage BPCrossBow)))

(event EventFireBolt
  ;[1 0.07208 0] Fire
  (CallFunction|SERVERFire))

(event EventTick
  (params (DeltaSeconds :type Float%20%28single-precision%29)))

(event Input|ActionEvents|InputActionTriggerRight
  (params (Key :type Key%20Structure :default "None"))
  ;[0 0 0] Comment
  (:Pressed
    (CallFunction|SERVERBeginPull))
  (:Released
    (CallFunction|SERVEREndPull)))

(fn ConstructionScript)

(fn GetControllerfromPC
  (bind _playercontroller (Class|INTCrossController|GetControllerPC(Message) (Pawn|GetController)))
  (return _playercontroller))

(fn GetControllerPC
  (return 0))