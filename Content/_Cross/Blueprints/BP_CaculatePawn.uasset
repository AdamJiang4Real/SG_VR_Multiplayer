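; BP_CaculatePawn is a VR pawn helper with a camera and right motion controller, apparently an unfinished position-calculation experiment.
; Tick forces VRCamera to world origin each frame, leaving its computed location difference unused.
; An unconnected chain would print the right controller's camera-relative position and pass it to the owning BP_Pawn.
; GetControllerFromPC returns the controller's PC message, while GetControllerPC is an empty stub.
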(event EventTick
  (params (DeltaSeconds :type Float%20%28single-precision%29))
  (bind _output_get (Variables|Default|Set1 (Transformation|GetWorldLocation (Variables|Default|GetVRCamera))))
  (bind _output_get_2 (Variables|Default|Set2 _output_get))
  (Variables|Default|Set2 (- _output_get_2 (Variables|Default|Get1)))
  (Transformation|SetWorldLocation (Variables|Default|GetVRCamera) "0, 0, 0" false false))

(event EventBeginPlay)

(fn ConstructionScript)

(fn GetControllerfromPC
  (bind _playercontroller (Class|INTCrossController|GetControllerPC(Message) (Pawn|GetController)))
  (return _playercontroller))

(fn GetControllerPC
  (return 0))