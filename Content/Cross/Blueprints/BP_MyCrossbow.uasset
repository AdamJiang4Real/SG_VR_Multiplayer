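; BP_MyCrossbow is a single-shot crossbow weapon with a toggleable bolt mesh and cyclable material variations.
; Fire checks ammo and a ready flag, clears both, then sends the character a message to fire the bolt.
; Reload restores both and messages the character to play the crossbow montage.
; TryFire and TryReload wrap these events without passing a character; older bolt-launch, sound and haptic logic remains disconnected.
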(event EventReload
  (params (Char :type BP%20Cross%20Pawn%20Object%20Reference))
  ;[1 1 1] Reload
  (Variables|Default|SetAmmo 1)
  (Class|INTCrossPawn|SpawnandPlayCrossMontage(Message) Char self)
  (Variables|Default|SetbCanFire true))

(event EventFire
  (params (Char :type BP%20Cross%20Pawn%20Object%20Reference))
  ;[1 1 1] Fire crossbow
  (if (and (> (Variables|Default|GetAmmo) 0) (Variables|Default|GetbCanFire))
    (Variables|Default|SetbCanFire false)
    (Class|INTCrossPawn|FireBolt(Message) Char)
    (Variables|Default|SetAmmo 0)))

(event EventBeginPlay
  ;[1 1 1] Setup
)

(fn ConstructionScript)

(fn SetBoltVisibility
  (params (Visible :type Boolean))
  ;[1 1 1] Show or hide the bolt
  (Rendering|SetVisibility (Variables|Default|GetBolt) Visible false))

(fn TryFire
  ;[1 1 1] Fire crossbow
  (CallFunction|Fire)
  (return true))

(fn TryReload
  ;[1 1 1] Start reload
  (CallFunction|Reload)
  (return true))

(fn SwitchMaterial
  ;[1 1 1] Switch Material
  (Math|Integer|IncrementInt (Variables|Default|GetMatIdx)
    (:%20%20
      (if (>= (Variables|Default|GetMatIdx) (Utilities|Array|Length (Variables|Default|GetMaterialVariations)))
        (Variables|Default|SetMatIdx 0))
      (Rendering|Material|SetMaterial (Variables|Default|GetCrossbowMesh) 0 (Utilities|Array|Get(acopy) (Variables|Default|GetMaterialVariations) (Variables|Default|GetMatIdx))))))